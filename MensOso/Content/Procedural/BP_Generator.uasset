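; BP_Generator is a procedural level generator that spawns room actors on a grid from a layout stored in a JSON file.
; On BeginPlay it reads the flattened matrix and its row and column counts, then walks every cell at 1000-unit spacing, skipping zeros.
; Each nonzero cell code selects an index range in the Rooms array, and SpawnRoom spawns a random class from that range at the cell position.
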(event EventBeginPlay
  (bind _outjsonobject (Class|JsonBlueprintFunctionLibrary|FromFile (Variables|Default|GetFile)))
  (Utilities|FlowControl|Sequence
    (:then_0
      (bind _outvalue (|GetJsonField _outjsonobject "matrix"))
      (Variables|Default|Setmatrix _outvalue))
    (:then_1
      (bind _outvalue_2 (|GetJsonField _outjsonobject "rows"))
      (Variables|Default|Setrows _outvalue_2))
    (:then_2
      (bind _outvalue_3 (|GetJsonField _outjsonobject "cols"))
      (Variables|Default|Setcols _outvalue_3))
    (:then_3
      (Variables|Default|Setcounter 0)
      (for _index (range 0 (- (Variables|Default|Getrows) 1))
        (for _index_2 (range 0 (- (Variables|Default|Getcols) 1))
          (bind _result (Math|Integer|IncrementInt (Variables|Default|Getcounter))
            (:%20%20
              (if (!= (Utilities|Array|Get(acopy) (Variables|Default|Getmatrix) (- _result 1)) 0)
                (bind _output_get (Variables|Default|SettransformPos (Math|Transform|MakeTransform (Math|Vector|MakeVector (Math|Conversions|ToFloat(Integer) (* _index 1000)) (Math|Conversions|ToFloat(Integer) (* _index_2 -1000)) 0.0) "0, 0, 0" "1.000000,1.000000,1.000000")))
                (switch int (- (Utilities|Array|Get(acopy) (Variables|Default|Getmatrix) (- _result 1)) 1)
                  (:0
                    (CallFunction|SpawnRoom 0 0 _output_get))
                  (:1
                    (CallFunction|SpawnRoom 1 3 _output_get))
                  (:2
                    (CallFunction|SpawnRoom 4 5 _output_get))
                  (:3
                    (CallFunction|SpawnRoom 6 9 _output_get))
                  (:4
                    (CallFunction|SpawnRoom 10 11 _output_get))
                  (:5
                    (CallFunction|SpawnRoom 12 12 _output_get))
                  (:6
                    (CallFunction|SpawnRoom 13 14 _output_get))
                  (:7
                    (CallFunction|SpawnRoom 15 15 _output_get))
                  (:8
                    (CallFunction|SpawnRoom 16 16 _output_get))
                  (:9
                    (CallFunction|SpawnRoom 17 17 _output_get)))))))))))

(fn ConstructionScript)

(fn SpawnRoom
  (params (minRange :type Integer) (maxRange :type Integer) (posToSpawn :type Transform))
  (Game|SpawnActorfromClass (Utilities|Array|Get(acopy) (Variables|Default|GetRooms) (Math|Random|RandomIntegerinRange minRange maxRange)) posToSpawn "Undefined" "MultiplyWithRoot" 0 0))