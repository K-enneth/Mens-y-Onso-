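; Procedural enemy spawner that has a random chance to spawn a small group of enemies when any actor overlaps it.
; An overlap while CanSpawn is set clears the flag and rolls for a spawn, while the next overlap only re-arms it.
; Each spawn picks a random class from Enemies and a random XY point within MinVal/MaxVal offsets of the spawner, at a hard-coded height.
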(event Collision|EventActorBeginOverlap
  (params (OtherActor :type Actor%20Object%20Reference))
  (bind _returnvalue (Transformation|GetActorTransform))
  (bind _minval (Variables|Default|GetminVal))
  (bind _maxval (Variables|Default|GetmaxVal))
  (if (Variables|Default|GetCanSpawn)
    (Variables|Default|SetCanSpawn false)
    (if (<= (Math|Random|RandomIntegerinRange 1 10) 3)
      (for _index (range 0 (Math|Random|RandomIntegerinRange 0 1))
        (Game|SpawnActorfromClass (Utilities|Array|Get(acopy) (Variables|Default|GetEnemies) (Math|Random|RandomIntegerinRange 0 (- (Utilities|Array|Length (Variables|Default|GetEnemies)) 1))) (Math|Transform|MakeTransform (Math|Vector|MakeVector (Math|Conversions|ToFloat(Integer) (Math|Random|RandomIntegerinRange (Math|Float|Truncate (- (.x (.location _returnvalue)) (.x _minval))) (Math|Float|Truncate (+ (.x (.location _returnvalue)) (.x _maxval))))) (Math|Conversions|ToFloat(Integer) (Math|Random|RandomIntegerinRange (Math|Float|Truncate (- (.y (.location _returnvalue)) (.y _minval))) (Math|Float|Truncate (+ (.y (.location _returnvalue)) (.y _maxval))))) 44.720464) "0, 0, 0" "1.000000,1.000000,1.000000") "Undefined" "MultiplyWithRoot" 0 0)))
    (else
      (Variables|Default|SetCanSpawn true))))

(fn ConstructionScript)