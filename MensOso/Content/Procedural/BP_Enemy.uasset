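; BP_Enemy is an enemy pawn that chases the player character and removes itself after a fixed two-minute lifetime.
; On BeginPlay, a cast of its NavMeshBoundsVolume reference gates the start of the chase, while a parallel sequence branch runs the destroy timer regardless.
; PlayerFollow drives AIMoveTo toward the first player's character and calls itself again on success or failure, keeping the pursuit continuous without Tick.
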(event Custom|PlayerFollow
  (AI|AIMoveTo self "0, 0, 0" (Game|GetPlayerCharacter 0) 0.5 false
    (:OnSuccess
      (CallFunction|PlayerFollow))
    (:OnFail
      (CallFunction|PlayerFollow))))

(event EventBeginPlay
  (Utilities|FlowControl|Sequence
    (:then_0
      (Utilities|Casting|CastToNavMeshBoundsVolumeClass "/Script/NavigationSystem.NavMeshBoundsVolume")
      (CallFunction|PlayerFollow))
    (:then_1
      (Utilities|FlowControl|Delay 1.2e+02)
      (Actor|DestroyActor))))

(fn ConstructionScript)