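; BP_EnemyManager is an actor that opens a referenced Door based on the loss of the enemies in its Enemies array.
; A looping one-second timer decrements a count, initialized to the array length, for each invalid entry and opens the door at zero.
; Invalid entries stay in the array, so each check counts them again.
; The manager destroys itself on any check that starts at zero.
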(event Custom|CheckEnemies
  (bind _totalenemies (Variables|Default|GetTotalEnemies))
  (if (== (Variables|Default|GetTotalEnemies) 0)
    (Actor|DestroyActor)
    (else
      (for _array_element (Variables|Default|GetEnemies)
        (Utilities|IsValid _array_element
          (:Is%20Not%20Valid
            (Math|Integer|DecrementInt _totalenemies
              (:%20%20
                (if (== _totalenemies 0)
                  (Default|OpenDoor (Variables|Default|GetDoor)))))))))))

(event EventBeginPlay
  (Utilities|Time|SetTimerbyEvent (delegate Custom|CheckEnemies) 1.0 true)
  (Variables|Default|SetTotalEnemies (Utilities|Array|Length (Variables|Default|GetEnemies))))

(fn ConstructionScript)