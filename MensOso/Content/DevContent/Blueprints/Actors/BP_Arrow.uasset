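; BP_Arrow is an arrow projectile actor that destroys itself one second after BeginPlay.
; Its overlap, FireArrow and DeactivateArrow events are empty.
; Disconnected nodes hold unused pooling-style logic that sets velocity, toggles the Arrow's collision and calls an OnDeactivateArrow dispatcher, so none of it runs.
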(event OnComponentBeginOverlap(Arrow)
  (params (OverlappedComponent :type Primitive%20Component%20Object%20Reference) (OtherActor :type Actor%20Object%20Reference) (OtherComp :type Primitive%20Component%20Object%20Reference) (OtherBodyIndex :type Integer) (bFromSweep :type Boolean) (SweepResult :type Hit%20Result%20Structure%20%28by%20ref%29)))

(event Custom|FireArrow
  (params (Velocity :type Vector)))

(event Custom|DeactivateArrow)

(event EventBeginPlay
  (Utilities|FlowControl|Delay 1.0)
  (Actor|DestroyActor))

(fn ConstructionScript)