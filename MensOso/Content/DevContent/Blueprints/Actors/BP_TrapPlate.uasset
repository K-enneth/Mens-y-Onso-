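; BP_TrapPlate is a floor plate actor that marks itself as correct or as a trap when a playable actor overlaps it.
; BeginPlay gives the static mesh a dynamic material instance so each plate can change color independently.
; On overlap with a BPI_Playable actor, the IsCorrect flag selects either a green tint or damage to that actor plus a red tint.
; The color is never reset afterward.
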(event EventBeginPlay
  (bind _returnvalue (Rendering|Material|CreateDynamicMaterialInstance (Rendering|Material|GetMaterial (Variables|Default|GetStaticMesh) 0) "None" "None" :!class /Script/Engine.KismetMaterialLibrary))
  (bind _output_get (Variables|Default|SetDynamicMaterial _returnvalue))
  (Rendering|Material|SetMaterial (Variables|Default|GetStaticMesh) 0 _output_get))

(event Collision|EventActorBeginOverlap
  (params (OtherActor :type Actor%20Object%20Reference))
  (if (Utilities|DoesObjectImplementInterface OtherActor "/Game/DevContent/Blueprints/BPI_Playable.BPI_Playable_C")
    (if (Variables|Default|GetIsCorrect)
      (Rendering|Material|SetVectorParameterValue (Variables|Default|GetDynamicMaterial) "color" "(R=0.000000,G=1.000000,B=0.081990,A=1.000000)" :!class /Script/Engine.MaterialInstanceDynamic)
      (else
        (Game|Damage|ApplyDamage OtherActor 1.0 0 0)
        (Rendering|Material|SetVectorParameterValue (Variables|Default|GetDynamicMaterial) "color" "(R=1.000000,G=0.000000,B=0.026037,A=1.000000)" :!class /Script/Engine.MaterialInstanceDynamic)))))

(fn ConstructionScript)