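; BP_CameraSwitch is an overlap trigger that toggles ActiveCamera between two locations.
; On BeginPlay it caches every BP_ThirdPersonCharacter.
; When a BPI_Playable actor overlaps, it moves all cached characters onto the trigger, then after a short delay a FlipFlop picks LocationA or LocationB for the camera.
; A DoOnce gates overlaps until the camera move resets it, so a non-playable overlap leaves it closed.
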(event EventBeginPlay
  (bind _outactors (Actor|GetAllActorsOfClass "/Game/DevContent/Blueprints/Characters/BP_ThirdPersonCharacter.BP_ThirdPersonCharacter_C"))
  (Variables|Default|SetCharacters _outactors))

(event Collision|EventActorBeginOverlap
  (params (OtherActor :type Actor%20Object%20Reference))
  (bind _activecamera (Variables|Default|GetActiveCamera))
  (Utilities|FlowControl|DoOnce false :!label _label
    (:Completed
      (if (Utilities|DoesObjectImplementInterface OtherActor "/Game/DevContent/Blueprints/BPI_Playable.BPI_Playable_C")
        (for _array_element (Variables|Default|GetCharacters)
          (Transformation|SetActorLocation _array_element (Transformation|GetActorLocation) false false)
          (Utilities|FlowControl|Delay 0.2)
          (Utilities|FlowControl|FlipFlop
            (:A
              (Transformation|SetActorLocation _activecamera (Variables|Default|GetLocationA) false false)
              (goto _label Reset))
            (:B
              (Transformation|SetActorLocation _activecamera (Variables|Default|GetLocationB) false false)
              (goto _label Reset))))))))

(fn ConstructionScript)