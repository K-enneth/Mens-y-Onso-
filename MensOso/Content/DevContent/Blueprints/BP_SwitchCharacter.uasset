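; Controller Blueprint that lets the player switch control between the BP_ThirdPersonCharacter instances in the level.
; BeginPlay caches all instances in an array and records the player's current character.
; The IA_Switch input calls SwitchCharacter, which selects the next array entry, wrapping to the first after the last, and possesses it.
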(event Input|EnhancedActionEvents|EnhancedInputActionIA_Switch
  (params (ActionValue :type Boolean) (ElapsedSeconds :type Float%20%28double-precision%29) (TriggeredSeconds :type Float%20%28double-precision%29) (InputAction :type Input%20Action%20Object%20Reference :default "/Game/DevContent/Input/Actions/IA_Switch.IA_Switch"))
  (:Started
    (CallFunction|SwitchCharacter)))

(event EventBeginPlay
  (bind _outactors (Actor|GetAllActorsOfClass "/Game/DevContent/Blueprints/Characters/BP_ThirdPersonCharacter.BP_ThirdPersonCharacter_C"))
  (Variables|Default|SetCharacters _outactors)
  (bind _asbp_third_person_character (Utilities|Casting|CastToBP_ThirdPersonCharacter (Game|GetPlayerCharacter 0)))
  (Variables|Default|SetCurrent%20Character _asbp_third_person_character))

(fn ConstructionScript)

(fn SwitchCharacter
  (LocalVariables|SetIndex (Utilities|Array|FindItem (Variables|Default|GetCharacters) (Variables|Default|GetCurrent%20Character)))
  (bind _output_get (LocalVariables|SetIndex (Math|Integer|SelectInt (+ (Utilities|Array|FindItem (Variables|Default|GetCharacters) (Variables|Default|GetCurrent%20Character)) 1) 0 (Utilities|Array|IsValidIndex (Variables|Default|GetCharacters) (+ (Utilities|Array|FindItem (Variables|Default|GetCharacters) (Variables|Default|GetCurrent%20Character)) 1)))))
  (bind _output_get_2 (Variables|Default|SetCurrent%20Character (Utilities|Array|Get(acopy) (Variables|Default|GetCharacters) _output_get)))
  (Pawn|Possess _output_get_2))