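; Sword-and-shield playable character Blueprint that adds a held block and a melee slash, both unavailable while dashing.
; Blocking plays a montage, slows walking and disables CanTakeDamage until release, and also prevents attacking.
; Attacking runs a box overlap ahead of the character with debug drawing, damages hit actors except PlayerCharacters, and plays a slash montage.
; IsAttacking gates repeat swings and clears after a delay inside the hit loop, so only when something is hit.
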(event Input|EnhancedActionEvents|EnhancedInputActionIA_Actions
  (params (ActionValue :type Boolean) (ElapsedSeconds :type Float%20%28double-precision%29) (TriggeredSeconds :type Float%20%28double-precision%29) (InputAction :type Input%20Action%20Object%20Reference :default "/Game/DevContent/Input/Actions/IA_Actions.IA_Actions"))
  (bind _charactermovement (Variables|Character|GetCharacterMovement))
  (:Started
    (if (not (Variables|Default|GetIsDashing))
      (Variables|Default|SetDoingAction true)
      (Variables|Default|SetCanTakeDamage false)
      (Variables|/Script/Engine.CharacterMovementComponent|SetMaxWalkSpeed _charactermovement 1e+02)
      (Animation|PlayAnimMontage "/Game/Models/Paladin/Sword_And_Shield_Block_Idle_Anim_mixamo_com_Montage.Sword_And_Shield_Block_Idle_Anim_mixamo_com_Montage" 1.0 "None")
      (Development|PrintString "Bloqueo")))
  (:Completed
    (Variables|Default|SetDoingAction false)
    (Variables|Default|SetCanTakeDamage true)
    (Variables|/Script/Engine.CharacterMovementComponent|SetMaxWalkSpeed _charactermovement 5e+02)))

(event Input|EnhancedActionEvents|EnhancedInputActionIA_Attack
  (params (ActionValue :type Boolean) (ElapsedSeconds :type Float%20%28double-precision%29) (TriggeredSeconds :type Float%20%28double-precision%29) (InputAction :type Input%20Action%20Object%20Reference :default "/Game/DevContent/Input/Actions/IA_Attack.IA_Attack"))
  (bind _returnvalue (Transformation|GetActorForwardVector))
  (bind _returnvalue_2 (Transformation|GetActorLocation))
  (bind _returnvalue_3 (* _returnvalue 1e+02))
  (bind _returnvalue_4 (+ _returnvalue_2 _returnvalue_3))
  (:Started
    (if (not (or (Variables|Default|GetDoingAction) (Variables|Default|GetIsDashing)))
      (if (not (Variables|Default|GetIsAttacking))
        (Variables|Default|SetIsAttacking true)
        (bind _outactors (Collision|BoxOverlapActors _returnvalue_4 "70.000000,100.000000,100.000000" (Utilities|Array|MakeArray "ObjectTypeQuery3" "ObjectTypeQuery1" "ObjectTypeQuery2") 0 (Variables|Default|GetPlayerCharacters) :!class /Script/Engine.KismetSystemLibrary))
        (Rendering|Debug|DrawDebugBox _returnvalue_4 "70.000000,100.000000,100.000000" "(R=0.971679,G=0.000000,B=1.000000,A=1.000000)" "0, 0, 0" 2.0 0.0)
        (Utilities|FlowControl|Sequence
          (:then_0
            (for _array_element _outactors
              (Game|Damage|ApplyDamage _array_element 1.0 0 0)
              (Utilities|FlowControl|Delay 0.5)
              (Variables|Default|SetIsAttacking false)))
          (:then_1
            (Animation|PlayAnimMontage "/Game/Models/Paladin/Sword_And_Shield_Slash_Montage.Sword_And_Shield_Slash_Montage" 1.0 "None")))))))

(fn ConstructionScript
  (|CallParentFunction))