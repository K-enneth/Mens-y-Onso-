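; Bow-wielding player character that adds aiming and shooting through Enhanced Input actions.
; Holding IA_Actions, unless dashing, enters an aim state that stops movement until release restores walk speed.
; Attacking while aiming spawns BP_Arrow at the Arrow1 component and immediately applies damage through a debug-drawn forward box trace that ignores player characters.
; A short delay on the attacking flag limits fire rate.
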(event Input|EnhancedActionEvents|EnhancedInputActionIA_Actions
  (params (ActionValue :type Boolean) (ElapsedSeconds :type Float%20%28double-precision%29) (TriggeredSeconds :type Float%20%28double-precision%29) (InputAction :type Input%20Action%20Object%20Reference :default "/Game/DevContent/Input/Actions/IA_Actions.IA_Actions"))
  (bind _charactermovement (Variables|Character|GetCharacterMovement))
  (:Started
    (if (not (Variables|Default|GetIsDashing))
      (Variables|Default|SetDoingAction true)
      (Variables|/Script/Engine.CharacterMovementComponent|SetMaxWalkSpeed _charactermovement 0.0)
      (Development|PrintString "Apuntando")))
  (:Completed
    (Variables|Default|SetDoingAction false)
    (Variables|/Script/Engine.CharacterMovementComponent|SetMaxWalkSpeed _charactermovement 5e+02)))

(event Input|EnhancedActionEvents|EnhancedInputActionIA_Attack
  (params (ActionValue :type Boolean) (ElapsedSeconds :type Float%20%28double-precision%29) (TriggeredSeconds :type Float%20%28double-precision%29) (InputAction :type Input%20Action%20Object%20Reference :default "/Game/DevContent/Input/Actions/IA_Attack.IA_Attack"))
  (bind _arrow1 (Variables|Default|GetArrow1))
  (bind _returnvalue (Transformation|GetWorldLocation _arrow1))
  (:Started
    (if (Variables|Default|GetDoingAction)
      (if (not (Variables|Default|GetIsAttacking))
        (Variables|Default|SetIsAttacking true)
        (Game|SpawnActorfromClass "/Game/DevContent/Blueprints/Actors/BP_Arrow.BP_Arrow_C" (Transformation|GetWorldTransform (Variables|Default|GetArrow1)) "AlwaysSpawn" "MultiplyWithRoot" 0 0)
        (bind _outhit (Collision|BoxTraceByChannel _returnvalue (+ _returnvalue (* (Math|Vector|GetForwardVector _arrow1) 1e+03)) "10.000000,10.000000,10.000000" "0, 0, 0" "TraceTypeQuery1" false (Variables|Default|GetPlayerCharacters) "ForDuration"))
        (Game|Damage|ApplyDamage (.HitActor (Collision|BreakHitResult _outhit)) 1.0 0 0)
        (Utilities|FlowControl|Delay 0.5)
        (Variables|Default|SetIsAttacking false)))))

(fn ConstructionScript
  (|CallParentFunction))