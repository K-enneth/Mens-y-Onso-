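; Inventory component that stores picked-up item info in a ten-slot Pickables array and provides the pause-menu inventory screen.
; BeginPlay creates the WBP_PauseInventory widget and loads it from the component.
; Show writes an item's info into the first slot with no valid image and a different name, refreshes the widget and destroys the item actor.
; IA_Pause displays the widget with cursor and UI-only input, and pauses the game.
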(event Custom|Show
  (params (Item :type BP%20Item%20Inventory%20Object%20Reference))
  (bind _iteminfo (Variables|/Game/DevContent/Blueprints/Actors/BP_ItemInventory.BP_ItemInventory_C|GetItemInfo Item))
  (bind (_array_element _array_index) (Utilities|Array|ForEachLoopwithBreak (Variables|Default|GetPickables) :!label _label)
    (:LoopBody
      (Utilities|IsValid Item
        (:Is%20Valid
          (if (not (Utilities|Enum|Equal(Enum) (.Name (Utilities|Struct|BreakS_InventoryItem _array_element)) (.Name (Utilities|Struct|BreakS_InventoryItem _iteminfo))))
            (Utilities|IsValid (.Image (Utilities|Struct|BreakS_InventoryItem _array_element))
              (:Is%20Not%20Valid
                (Utilities|Array|SetArrayElem (Variables|Default|GetPickables) _array_index _iteminfo)
                (Default|LoadInventory (Variables|Default|GetWidget) self)
                (Actor|DestroyActor Item)
                (goto _label Break)))))))))

(event Input|EnhancedActionEvents|EnhancedInputActionIA_Pause
  (params (ActionValue :type Boolean) (ElapsedSeconds :type Float%20%28double-precision%29) (TriggeredSeconds :type Float%20%28double-precision%29) (InputAction :type Input%20Action%20Object%20Reference :default "/Game/DevContent/Input/Actions/IA_Pause.IA_Pause"))
  (bind _returnvalue (Game|GetPlayerController 0))
  (:Started
    (Development|PrintString "Hello")
    (Variables|/Script/Engine.PlayerController|SetbShowMouseCursor _returnvalue true)
    (UserInterface|Viewport|AddtoViewport (Variables|Default|GetWidget) 0)
    (Input|SetInputModeUIOnly _returnvalue 0 "DoNotLock" false)
    (Game|SetGamePaused true)))

(event EventBeginPlay
  (bind _returnvalue (UserInterface|CreateWidget "/Game/DevContent/Widgets/WBP_PauseInventory.WBP_PauseInventory_C"))
  (Variables|Default|SetWidget _returnvalue)
  (Utilities|Array|Resize (Variables|Default|GetPickables) 10)
  (Default|LoadInventory (Variables|Default|GetWidget) self))