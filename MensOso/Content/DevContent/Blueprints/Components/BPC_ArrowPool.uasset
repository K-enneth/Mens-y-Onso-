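; BPC_ArrowPool is an actor component meant to pool BP_Arrow actors on its owner for reuse.
; ReturnArrow moves a given arrow back to the owner's location and attaches it there.
; The pool-filling logic, which spawns collision-disabled, attached arrows and binds ReturnArrow to their deactivate dispatcher, is disconnected.
; BeginPlay is empty, so the component never populates the pool itself.
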(event Custom|Return%20Arrow
  (params (Arrow :type BP%20Arrow%20Object%20Reference))
  (bind _returnvalue (Components|GetOwner))
  (Transformation|SetActorLocation Arrow (Transformation|GetActorLocation _returnvalue) false false)
  (Transformation|AttachActorToActor Arrow _returnvalue "None" "KeepWorld" "KeepWorld" "KeepWorld" true))

(event EventBeginPlay)