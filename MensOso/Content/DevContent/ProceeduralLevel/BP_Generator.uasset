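; BP_Generator builds a grid-based level at BeginPlay by spawning room actors from a layout stored in a JSON file.
; It reads the column count, row count and flat matrix, then walks every cell with a running counter.
; Non-zero cells are placed on a 600-unit grid, and values 1 and 2 call SpawnRoom, whose random index range currently resolves to Rooms entry 0 or 1 respectively.
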(event EventBeginPlay
  ;[1 0.4803 0.1953] Lectura del archivo json para crear los niveles
  (bind _outjsonobject (Class|JsonBlueprintFunctionLibrary|FromFile (Variables|Default|GetFile)))
  (Utilities|FlowControl|Sequence
    (:then_0
      ;[0.2782 0.7562 1] Asignacion de Variables para la lectura de la matriz
      (bind _outvalue (|GetJsonField _outjsonobject "cols"))
      (Variables|Default|Setcols _outvalue))
    (:then_1
      (bind _outvalue_2 (|GetJsonField _outjsonobject "rows"))
      (Variables|Default|Setrows _outvalue_2))
    (:then_2
      (bind _outvalue_3 (|GetJsonField _outjsonobject "matrix"))
      (Variables|Default|Setmatrix _outvalue_3))
    (:then_3
      ;[0.1323 0.07292 0.875] Recorriendo la matriz en todos sus valores
      (Variables|Default|Setcounter 0)
      (for _index (range 0 (- (Variables|Default|Getrows) 1))
        (for _index_2 (range 0 (- (Variables|Default|Getcols) 1))
          (bind _result (Math|Integer|IncrementInt (Variables|Default|Getcounter))
            (:%20%20
              ;[0.875 0.5661 0.1413] Logica para definir que cuartos se van a spawnear
              (if (!= (Utilities|Array|Get(acopy) (Variables|Default|Getmatrix) (- _result 1)) 0)
                (bind _output_get (Variables|Default|Setposition (Math|Transform|MakeTransform (Math|Vector|MakeVector (Math|Conversions|ToFloat(Integer) (* _index -600)) (Math|Conversions|ToFloat(Integer) (* _index_2 600)) 0.0) "0, 0, 0" "1.000000,1.000000,1.000000")))
                (switch int (- (Utilities|Array|Get(acopy) (Variables|Default|Getmatrix) (- _result 1)) 1)
                  (:0
                    (CallFunction|SpawnRoom 0 0 _output_get))
                  (:1
                    (CallFunction|SpawnRoom 1 1 _output_get)))))))))))

(fn ConstructionScript)

(fn SpawnRoom
  (params (minRange :type Integer) (maxRange :type Integer) (posotion :type Transform))
  (Game|SpawnActorfromClass (Utilities|Array|Get(acopy) (Variables|Default|Getrooms) (Math|Random|RandomIntegerinRange minRange maxRange)) posotion "Undefined" "MultiplyWithRoot" 0 0))